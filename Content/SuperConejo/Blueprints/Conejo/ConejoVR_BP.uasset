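; VR player Blueprint for the rabbit (Conejo) that throws chocolate balls from both motion controllers and reacts to being hit.
; BeginPlay enables the HMD, and each hand's input spawns a ball just ahead of its controller and calls Lanzar, with the right hand using the physics variant.
; When Colision overlaps a BolaChocolate, it prints a hit message, destroys the ball and plays haptics on the left controller.
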(event OnComponentBeginOverlap(Colision)
  (params (OverlappedComponent :type Primitive%20Component%20Object%20Reference) (OtherActor :type Actor%20Object%20Reference) (OtherComp :type Primitive%20Component%20Object%20Reference) (OtherBodyIndex :type Integer) (bFromSweep :type Boolean) (SweepResult :type Hit%20Result%20Structure%20%28by%20ref%29))
  (bind _asbola_chocolate (Utilities|Casting|CastToBolaChocolate OtherActor))
  (Development|PrintText "Golpe")
  (Actor|DestroyActor _asbola_chocolate)
  (Class|PlayerController|PlayHapticEffect (Game|GetPlayerController 0) "/Game/ControllerSetup/ForceFeedbacks/GolpeadoHapticFeedbackEffect_Curve.GolpeadoHapticFeedbackEffect_Curve" "Left" 1.0 false))

(event EventBeginPlay
  (Class|HeadMountedDisplayFunctionLibrary|EnableHMD true))

(event Collision|EventActorBeginOverlap
  (params (OtherActor :type Actor%20Object%20Reference)))

(event EventTick
  (params (DeltaSeconds :type Float%20%28single-precision%29)))

(event Input|ActionEvents|InputActionLanzarBolitaRight
  (params (Key :type Key%20Structure :default "AnyKey"))
  (bind _rightcontroller (Variables|Default|GetRightController))
  (:Pressed
    (bind _returnvalue (Game|SpawnActorfromClass "/Game/SuperConejo/Blueprints/BolasChocolate/BolaChocolateFisica_BP.BolaChocolateFisica_BP_C" (Math|Transform|MakeTransform (+ (Transformation|GetWorldLocation _rightcontroller) (* (Math|Vector|GetForwardVector _rightcontroller) 1e+01)) (Transformation|GetWorldRotation _rightcontroller)) "Undefined" self (Variables|Default|GetInstigator)))
    (Class|BolaChocolate|Lanzar _returnvalue)))

(event Input|ActionEvents|InputActionLanzarBolitaLeft
  (params (Key :type Key%20Structure :default "AnyKey"))
  (bind _leftcontroller (Variables|Default|GetLeftController))
  (:Pressed
    (bind _returnvalue (Game|SpawnActorfromClass "/Game/SuperConejo/Blueprints/BolasChocolate/BolaChocolate_BP.BolaChocolate_BP_C" (Math|Transform|MakeTransform (+ (Transformation|GetWorldLocation _leftcontroller) (* (Math|Vector|GetForwardVector _leftcontroller) 1e+01)) (Transformation|GetWorldRotation _leftcontroller)) "Undefined" self (Variables|Default|GetInstigator)))
    (Class|BolaChocolate|Lanzar _returnvalue)))

(fn ConstructionScript)