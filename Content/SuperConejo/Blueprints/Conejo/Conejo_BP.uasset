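; Player rabbit Blueprint for SuperConejo that throws chocolate balls and handles run input.
; The Lanzar input calls Lanzar2, which spawns a TipoBolaChocolate at the PuntoLanzamiento transform with itself as owner, then calls Lanzar on that ball.
; The Correr input only prints debug text, intentionally replacing the code-side binding without calling the parent.
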(event EventBeginPlay)

(event Collision|EventActorBeginOverlap
  (params (OtherActor :type Actor%20Object%20Reference)))

(event EventTick
  (params (DeltaSeconds :type Float%20%28single-precision%29)))

(event Input|ActionEvents|InputActionCorrer
  (params (Key :type Key%20Structure :default "AnyKey"))
  ;[0.065 0.065 0.065] En este caso modifica el bind del codigo, para que jejecute esta funcion, en este caso no hay llamada a la funcion del padre
  (:Pressed
    (Development|PrintText "CorriendoBP")))

(event Input|ActionEvents|InputActionLanzar
  (params (Key :type Key%20Structure :default "AnyKey"))
  (:Pressed
    (CallFunction|Lanzar2)))

(fn ConstructionScript)

(fn Lanzar2
  (bind _punto_lanzamiento (Variables|Default|GetPunto%20Lanzamiento))
  (bind _returnvalue (Game|SpawnActorfromClass (Variables|Default|GetTipoBolaChocolate) (Math|Transform|MakeTransform (Transformation|GetWorldLocation _punto_lanzamiento) (Transformation|GetWorldRotation _punto_lanzamiento)) "Undefined" self (Variables|Default|GetInstigator)))
  (Class|BolaChocolate|Lanzar _returnvalue))