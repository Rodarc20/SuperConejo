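; BolaChocolateFisica_BP is a chocolate ball actor, apparently physics-based, that currently only logs collision debug text.
; It has a Bola mesh and a separate Colision component, and Bola's begin-overlap prints the other actor's name.
; Bola's hit and Colision's overlap handlers are empty, with their debug prints disconnected.
; Author notes warn that the two components also detect each other's overlaps.
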(event OnComponentHit(Bola)
  (params (HitComponent :type Primitive%20Component%20Object%20Reference) (OtherActor :type Actor%20Object%20Reference) (OtherComp :type Primitive%20Component%20Object%20Reference) (NormalImpulse :type Vector :default "0, 0, 0") (Hit :type Hit%20Result%20Structure%20%28by%20ref%29))
  ;[1 1 1] Nada
)

(event OnComponentBeginOverlap(Bola)
  (params (OverlappedComponent :type Primitive%20Component%20Object%20Reference) (OtherActor :type Actor%20Object%20Reference) (OtherComp :type Primitive%20Component%20Object%20Reference) (OtherBodyIndex :type Integer) (bFromSweep :type Boolean) (SweepResult :type Hit%20Result%20Structure%20%28by%20ref%29))
  ;[1 1 1] Detecta a los otros actores, pero tambien al componente colision de este actor
  (Development|PrintText (Utilities|Text|ToText(String) (Utilities|String|Append "OverlapBola with " (Utilities|GetObjectName OtherActor)))))

(event OnComponentBeginOverlap(Colision)
  (params (OverlappedComponent :type Primitive%20Component%20Object%20Reference) (OtherActor :type Actor%20Object%20Reference) (OtherComp :type Primitive%20Component%20Object%20Reference) (OtherBodyIndex :type Integer) (bFromSweep :type Boolean) (SweepResult :type Hit%20Result%20Structure%20%28by%20ref%29))
  ;[1 1 1] Tambien detecta a los otrso actores, y al statich mesh de este actor, util masomnos, tener cuidado
)

(event EventBeginPlay)

(event Collision|EventActorBeginOverlap
  (params (OtherActor :type Actor%20Object%20Reference)))

(event EventTick
  (params (DeltaSeconds :type Float%20%28single-precision%29)))

(fn ConstructionScript)