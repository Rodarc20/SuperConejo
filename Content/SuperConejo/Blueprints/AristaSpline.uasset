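; AristaSpline is an actor that lays three preset spline mesh segments along its Spline component, apparently forming an edge.
; On BeginPlay, each segment's start and end snap to consecutive local spline points, the first four in total, without passing the spline's tangents.
; Disconnected drafts in the event graph and construction script would generate thin cylinder segments dynamically from hardcoded points, but never run.
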(event EventBeginPlay
  (bind _spline (Variables|Default|GetSpline))
  (bind _spline_2 (Variables|Default|GetSpline))
  (bind _spline_3 (Variables|Default|GetSpline))
  (SplineMesh|SetStartandEnd (Variables|Default|GetSplineMesh) (.Location (Spline|GetLocationandTangentatSplinePoint _spline_2 0 "Local")) "0, 0, 0" (.Location (Spline|GetLocationandTangentatSplinePoint _spline_2 1 "Local")) "0, 0, 0" true :!class /Script/Engine.SplineMeshComponent)
  (SplineMesh|SetStartandEnd (Variables|Default|GetSplineMesh1) (.Location (Spline|GetLocationandTangentatSplinePoint _spline_3 1 "Local")) "0, 0, 0" (.Location (Spline|GetLocationandTangentatSplinePoint _spline_3 2 "Local")) "0, 0, 0" true :!class /Script/Engine.SplineMeshComponent)
  (SplineMesh|SetStartandEnd (Variables|Default|GetSplineMesh2) (.Location (Spline|GetLocationandTangentatSplinePoint _spline 2 "Local")) "0, 0, 0" (.Location (Spline|GetLocationandTangentatSplinePoint _spline 3 "Local")) "0, 0, 0" true :!class /Script/Engine.SplineMeshComponent))

(event Collision|EventActorBeginOverlap
  (params (OtherActor :type Actor%20Object%20Reference)))

(event EventTick
  (params (DeltaSeconds :type Float%20%28single-precision%29)))

(fn ConstructionScript)